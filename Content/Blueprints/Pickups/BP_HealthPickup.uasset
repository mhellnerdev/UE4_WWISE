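; BP_HealthPickup is a health pickup that a BP_Marine collects by overlapping it, provided the marine's health is not full.
; On collection it stores its location and scale, plays a sound, then runs a timeline that lerps it toward the player pawn while shrinking it to zero.
; When the timeline finishes, it adds health to the marine and destroys itself.
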(event EventBeginPlay)

(event Collision|EventActorBeginOverlap
  (params (OtherActor :type Actor%20Object%20Reference))
  (bind _asbp_marine (Utilities|Casting|CastToBP_Marine OtherActor))
  (CallFunction|StoreStartingValuesforTimeline)
  (if (not (Default|IsHealthFull _asbp_marine))
    (Audio|PlaySound2D "/Game/Sounds/FACF-chord-smoothring_transposed+6.FACF-chord-smoothring_transposed+6" 1.0 1.0 0.0 0 0)
    (bind (_direction _collectionprogress _scaleprogress) (Timeline|CollectionTimeline Play)
      (:Update
        (CallFunction|MovetoPlayer _collectionprogress)
        (CallFunction|ScalePickup _scaleprogress))
      (:Finished
        (Default|AddHealth _asbp_marine (Variables|Default|GetHealthPickupAmount))
        (Actor|DestroyActor)))))

(event EventTick
  (params (DeltaSeconds :type Float%20%28single-precision%29)))

(fn ConstructionScript)

(fn MovetoPlayer
  (params (Alpha :type Float%20%28single-precision%29))
  (Transformation|SetActorLocation (Math|Vector|Lerp(Vector) (Variables|Default|GetStartLocation) (Transformation|GetActorLocation (Game|Player|GetPlayerPawn 0)) Alpha) false false))

(fn ScalePickup
  (params (Alpha :type Float%20%28single-precision%29))
  (Transformation|SetActorScale3D (Math|Vector|Lerp(Vector) (Variables|Default|GetstartScale) "0, 0, 0" Alpha)))

(fn StoreStartingValuesforTimeline
  (Variables|Default|SetStartLocation (Transformation|GetActorLocation))
  (Variables|Default|SetstartScale (Transformation|GetActorScale3D)))